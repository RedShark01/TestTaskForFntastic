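; BP_Nest is a numbered nest actor that spawns turtles bound for a linked Destination.
; Its construction script writes Index onto its own label and the Destination's, visually pairing the two.
; SpawnTurtle spawns TurtleClass at SpawnPoint, passing itself as start point along with Destination and Index, then plays a button-press sound.
; Each tick, the index and name texts rotate to face the player.
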(event EventTick
  (params (DeltaSeconds :type Float%20%28single-precision%29))
  ;[1 1 1] Rotate Index and Name to Player
  (CallFunction|RotateComponenttoPlayer (Variables|Default|GetIndexText))
  (CallFunction|RotateComponenttoPlayer (Variables|Default|GetNameText)))

(fn ConstructionScript
  (bind _index (Variables|Settings|GetIndex))
  (bind _returnvalue (Utilities|Text|ToText(Integer) _index))
  (Rendering|Components|TextRender|SetText (Variables|Default|GetIndexText) _returnvalue)
  (Rendering|Components|TextRender|SetText (Variables|/Game/Blueprints/BP_Destination.BP_Destination_C|GetIndexText (Variables|Settings|GetDestination)) _returnvalue))

(fn SpawnTurtle
  (bind _spawnpoint (Variables|Default|GetSpawnPoint))
  (Game|SpawnActorfromClass (Variables|Settings|GetTurtleClass) (Math|Transform|MakeTransform (Transformation|GetWorldLocation _spawnpoint) (Transformation|GetWorldRotation _spawnpoint) "1,1,1") "Undefined" self (Variables|Settings|GetDestination) self (Variables|Settings|GetIndex) 0)
  (Audio|PlaySoundatLocation "/Game/Assets/Sounds/ButtonPress.ButtonPress" (Transformation|GetActorLocation) "0, 0, 0" 1.0 1.0 0.0 0 0 0))