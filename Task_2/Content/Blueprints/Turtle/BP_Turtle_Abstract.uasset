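; Abstract base Character for turtles that walk from a start point to a destination actor, showing their index on floating text.
; After a short BeginPlay delay it sets the text and starts AI MoveTo if both points are valid; on success it notifies the destination and destroys itself.
; An empty ChangeTurtleBehavior event, called as movement begins, serves as the override hook for subclasses.
; Tick keeps the text rotated toward the player.
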(event Custom|MoveToDestination
  ;[1 1 1] SimpleMoveToActor
  (AI|AIMoveTo self "0, 0, 0" (Variables|Default|GetDestination) 5.0 false
    (:then
      (CallFunction|ChangeTurtleBehavior))
    (:OnSuccess
      (Class|BPIStadartInterface|Finish(Message) (Variables|Default|GetDestination))
      (Actor|DestroyActor))))

(event Custom|ChangeTurtleBehavior
  ;[1 1 1] Abstract Event
)

(event EventTick
  (params (DeltaSeconds :type Float%20%28single-precision%29))
  ;[1 1 1] RotateTextToPlayer
  (CallFunction|RotateComponenttoPlayer (Variables|Default|GetIndexText)))

(event EventBeginPlay
  ;[1 1 1] BeginPlay
  (Utilities|FlowControl|Delay 0.01)
  (Rendering|Components|TextRender|SetText (Variables|Default|GetIndexText) (Utilities|Text|ToText(Integer) (Variables|Default|GetIndex)))
  (if (and (Utilities|IsValid (Variables|Default|GetDestination)) (Utilities|IsValid (Variables|Default|GetPointBegin)))
    (CallFunction|MovetoDestination)))

(fn ConstructionScript
  (Variables|/Script/Engine.CharacterMovementComponent|SetMaxWalkSpeed (Variables|Character|GetCharacterMovement) (Variables|Default|GetStandardWalkSpeed)))