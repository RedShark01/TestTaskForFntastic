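; BP_Button is an interactable button tied to a Nest that spawns a turtle from that nest when used.
; The construction script writes the nest's index onto its index text component.
; Each tick it rotates the index and name text components to face the player.
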(event EventInteract
  (Default|SpawnTurtle (Variables|Settings|GetNest)))

(event EventTick
  (params (DeltaSeconds :type Float%20%28single-precision%29))
  (CallFunction|RotateComponenttoPlayer (Variables|Default|GetIndexText))
  (CallFunction|RotateComponenttoPlayer (Variables|Default|GetNameText)))

(fn ConstructionScript
  (Rendering|Components|TextRender|SetText (Variables|Default|GetIndexText) (Utilities|Text|ToText(Integer) (Variables|/Game/Blueprints/BP_Nest.BP_Nest_C|GetIndex (Variables|Settings|GetNest)))))