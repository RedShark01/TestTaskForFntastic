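; BP_Destination is a destination marker actor that shows index and name text and celebrates when finished.
; Each Tick passes both text components to RotateComponentToPlayer so they turn toward the player.
; The Finish event plays a sound at the actor's location and spawns an explosion particle effect slightly above it.
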(event EventTick
  (params (DeltaSeconds :type Float%20%28single-precision%29))
  ;[1 1 1] Rotate index and text to player
  (CallFunction|RotateComponenttoPlayer (Variables|Default|GetIndexText))
  (CallFunction|RotateComponenttoPlayer (Variables|Default|GetNameText)))

(event EventFinish
  (bind _returnvalue (Transformation|GetActorLocation))
  (bind (_x _y _z) (Math|Vector|BreakVector _returnvalue))
  ;[1 1 1] Finish Effects
  (Audio|PlaySoundatLocation "/Game/Assets/Sounds/FinishSound.FinishSound" _returnvalue "0, 0, 0" 1.0 1.0 0.0 0 0 0)
  (Effects|SpawnEmitteratLocation "/Game/Assets/StarterContent/Particles/P_Explosion.P_Explosion" (Math|Vector|MakeVector _x _y (+ _z 1e+02))))

(fn ConstructionScript)